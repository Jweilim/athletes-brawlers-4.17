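; Main camera actor for the fighting game, which makes itself the view target and frames both players.
; BeginPlay finds the two selected characters, centers on their Y midpoint and sets a look-at rotation.
; While GamePlay is true, Tick takes both players from BP_Global_Controller, applies spring arm and rotation setup once, then follows their Y midpoint.
; Leaving gameplay re-arms that one-time setup.
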(event EventTick
  (params (DeltaSeconds :type Float%20%28single-precision%29))
  (bind _returnvalue (Transformation|GetActorLocation))
  (bind _springarm (Variables|Default|GetSpringArm))
  (bind (_x _y _z) (Math|Vector|BreakVector _returnvalue))
  ;[1 1 1] Condition
  (if (Variables|Default|GetGamePlay)
    ;[1 1 1] Default - Again
    (Game|Player|SetViewTargetwithBlend (Game|GetPlayerController 0) self 0.0 "VTBlend_Linear" 0.0 false)
    ;[1 1 1] Cast Player01 and Player02 GlobalController
    (bind _asbp_global_controller (Utilities|Casting|CastToBP_Global_Controller (Game|GetPlayerController 0)))
    (Variables|Default|SetPlayer01 (Variables|/Game/Fight_Game/Blueprints/BP_Global_Controller.BP_Global_Controller_C|GetPlayer01 _asbp_global_controller))
    (Variables|Default|SetPlayer02 (Variables|/Game/Fight_Game/Blueprints/BP_Global_Controller.BP_Global_Controller_C|GetPlayer02 _asbp_global_controller))
    (Utilities|FlowControl|Sequence
      (:then_0
        ;[1 1 1] Reset for currect Rotation
        (Utilities|FlowControl|DoOnce false :!label _label
          (:Completed
            (Variables|/Script/Engine.SpringArmComponent|SetTargetArmLength _springarm 3e+02)
            (Transformation|SetRelativeRotation _springarm "45.000000, 0, 0" false false)
            (Transformation|SetWorldLocationAndRotation (Variables|Default|GetDefaultSceneRoot) (Math|Vector|MakeVector (+ (.X (Math|Vector|BreakVector (.Location (Math|Transform|BreakTransform (Transformation|GetActorTransform (Variables|Default|GetPlayer01)))))) 3e+01) -1.8e+02 (+ (.Z (Math|Vector|BreakVector (.Location (Math|Transform|BreakTransform (Transformation|GetActorTransform (Variables|Default|GetPlayer01)))))) 25.0)) "0.000000,-180.000000, 0" false false)
            (bind _output_get (Variables|Default|SetDefaultRotator (Math|Rotator|FindLookatRotation (Math|Vector|MakeVector _x (|((a+b)/2) (.Y (Math|Vector|BreakVector (Transformation|GetActorLocation (Variables|Default|GetPlayer01)))) (.Y (Math|Vector|BreakVector (Transformation|GetActorLocation (Variables|Default|GetPlayer02))))) _z) (Math|Vector|MakeVector (|((a+b)/2) (.X (Math|Vector|BreakVector (Transformation|GetActorLocation (Variables|Default|GetPlayer01)))) (.Z (Math|Vector|BreakVector (Transformation|GetActorLocation (Variables|Default|GetPlayer01))))) (|((a+b)/2) (.Y (Math|Vector|BreakVector (Transformation|GetActorLocation (Variables|Default|GetPlayer01)))) (.Y (Math|Vector|BreakVector (Transformation|GetActorLocation (Variables|Default|GetPlayer02))))) (|((a+b)/2) (.X (Math|Vector|BreakVector (Transformation|GetActorLocation (Variables|Default|GetPlayer02)))) (.Z (Math|Vector|BreakVector (Transformation|GetActorLocation (Variables|Default|GetPlayer02)))))))))
            (Transformation|SetActorRotation _output_get))))
      (:then_1
        ;[1 1 1] Follow to player same time
        (Transformation|SetActorLocation (Math|Vector|MakeVector _x (|((a+b)/2) (.Y (Math|Vector|BreakVector (Transformation|GetActorLocation (Variables|Default|GetPlayer01)))) (.Y (Math|Vector|BreakVector (Transformation|GetActorLocation (Variables|Default|GetPlayer02))))) _z) false false)))
    (else
      (goto _label Reset))))

(event EventBeginPlay
  (bind _returnvalue (Transformation|GetActorLocation))
  (bind (_x _y _z) (Math|Vector|BreakVector _returnvalue))
  ;[1 1 1] StartGame(Default)
  (Game|Player|SetViewTargetwithBlend (Game|GetPlayerController 0) self 0.0 "VTBlend_Linear" 0.0 false)
  (Utilities|FlowControl|DoOnce false
    (:Completed
      ;[1 1 1] Cast Player01 and Player02 Scene
      (bind _asbp_select_player_02 (Utilities|Casting|CastToBP_Select_Player02Class "/Game/Fight_Game/Blueprints/BP_Select_Player01.BP_Select_Player01_C"))
      (bind _outactors (Actor|GetAllActorsOfClass _asbp_select_player_02))
      (bind _asbp_select_player_01 (Utilities|Casting|CastToBP_Select_Player01Class "/Game/Fight_Game/Blueprints/BP_Select_Player02.BP_Select_Player02_C"))
      (bind _outactors_2 (Actor|GetAllActorsOfClass _asbp_select_player_01))
      (Variables|Default|SetPlayer01 (Utilities|Array|Get(acopy) _outactors))
      (Variables|Default|SetPlayer02 (Utilities|Array|Get(acopy) _outactors_2))
      ;[1 1 1] Reset for currect Rotation
      (Transformation|SetActorLocation (Math|Vector|MakeVector _x (|((a+b)/2) (.Y (Math|Vector|BreakVector (Transformation|GetActorLocation (Variables|Default|GetPlayer01)))) (.Y (Math|Vector|BreakVector (Transformation|GetActorLocation (Variables|Default|GetPlayer02))))) _z) false false)
      (Transformation|SetActorRotation (Math|Rotator|FindLookatRotation (Math|Vector|MakeVector _x (|((a+b)/2) (.Y (Math|Vector|BreakVector (Transformation|GetActorLocation (Variables|Default|GetPlayer01)))) (.Y (Math|Vector|BreakVector (Transformation|GetActorLocation (Variables|Default|GetPlayer02))))) _z) (Math|Vector|MakeVector (|((a+b)/2) (.X (Math|Vector|BreakVector (Transformation|GetActorLocation (Variables|Default|GetPlayer01)))) (.Z (Math|Vector|BreakVector (Transformation|GetActorLocation (Variables|Default|GetPlayer01))))) (|((a+b)/2) (.Y (Math|Vector|BreakVector (Transformation|GetActorLocation (Variables|Default|GetPlayer01)))) (.Y (Math|Vector|BreakVector (Transformation|GetActorLocation (Variables|Default|GetPlayer02))))) (|((a+b)/2) (.X (Math|Vector|BreakVector (Transformation|GetActorLocation (Variables|Default|GetPlayer02)))) (.Z (Math|Vector|BreakVector (Transformation|GetActorLocation (Variables|Default|GetPlayer02)))))))))))

(fn ConstructionScript)