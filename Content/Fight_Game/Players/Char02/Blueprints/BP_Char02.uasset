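; Fighter character Blueprint for Char02, which assigns itself as Player 1 or 2 from its starting Y position.
; Tick zeroes acceleration while crouching and polls the fight menu widget to drive costume and animation state.
; A Player 2 color-change flag applies a yellow body tint through a dynamic material.
; Menu ready flags trigger a looping ready animation, and starting play hands the mesh to the character's Animation Blueprint.
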(event Custom|Color
  ;[1 1 1] Change Color Costume
  (bind _returnvalue (Rendering|Material|CreateDynamicMaterialInstance (Variables|Character|GetMesh) 0 "/Game/Fight_Game/Players/Char01/Material/M_Char01.M_Char01" :!class /Script/Engine.PrimitiveComponent))
  (bind _output_get (Variables|Default|SetDynamicColor _returnvalue))
  (Rendering|Material|SetVectorParameterValue _output_get "BodyColor" "(R=1.000000,G=0.922931,B=0.000000,A=1.000000)" :!class /Script/Engine.MaterialInstanceDynamic))

(event EventTick
  (params (DeltaSeconds :type Float%20%28single-precision%29))
  (bind _mesh (Variables|Character|GetMesh))
  (bind _charactermovement (Variables|Character|GetCharacterMovement))
  (Utilities|FlowControl|Sequence
    (:then_0
      ;[1 1 1] Crouching - Stop and Restore Acceleration
      (if (AI|Components|NavMovement|IsCrouching _charactermovement)
        (Variables|/Script/Engine.CharacterMovementComponent|SetMaxAcceleration _charactermovement 0.0)
        (else
          (Variables|/Script/Engine.CharacterMovementComponent|SetMaxAcceleration _charactermovement 2048.0))))
    (:then_1
      ;[1 1 1] Look for Same Character Costume
      (bind _asfight_game_menu (CallFunction|CastFightGameMenu))
      (if (Variables|/Game/Fight_Game/HUD/Widget_FightGame_Menu.Widget_FightGame_Menu_C|GetP2_ChangeColor _asfight_game_menu)
        (if (not (Variables|Default|GetPlayer01?))
          (if (Variables|/Game/Fight_Game/HUD/Widget_FightGame_Menu.Widget_FightGame_Menu_C|GetPlay_Game _asfight_game_menu)
            (Utilities|FlowControl|DoOnce false
              (:Completed
                (CallFunction|Color)))
            (else
              (CallFunction|Color))))))
    (:then_2
      ;[1 1 1] Animation Select
      (bind _asfight_game_menu_2 (CallFunction|CastFightGameMenu))
      (Utilities|FlowControl|Sequence
        (:then_0
          (if (Variables|/Game/Fight_Game/HUD/Widget_FightGame_Menu.Widget_FightGame_Menu_C|GetP01_AnimReady _asfight_game_menu_2)
            (if (Variables|Default|GetPlayer01?)
              (Utilities|FlowControl|DoOnce false :!label _label
                (:Completed
                  (Components|Animation|PlayAnimation (Variables|Character|GetMesh) "/Game/Fight_Game/Players/Char01/Animations/Char_Ready.Char_Ready" true))))))
        (:then_1
          (if (Variables|/Game/Fight_Game/HUD/Widget_FightGame_Menu.Widget_FightGame_Menu_C|GetP02_AnimReady _asfight_game_menu_2)
            (if (not (Variables|Default|GetPlayer01?))
              (goto _label))))))
    (:then_3
      ;[1 1 1] Rstore Control Animation
      (bind _asfight_game_menu_3 (CallFunction|CastFightGameMenu))
      (if (Variables|/Game/Fight_Game/HUD/Widget_FightGame_Menu.Widget_FightGame_Menu_C|GetPlay_Game _asfight_game_menu_3)
        (Utilities|FlowControl|DoOnce false :!label _label_2
          (:Completed
            (Components|Animation|SetAnimationMode _mesh "AnimationBlueprint")
            (Components|SkeletalMesh|SetAnimInstanceClass _mesh "/Game/Fight_Game/Players/Char01/Blueprints/Char_AnimBP.Char_AnimBP_C")))
        (else
          (goto _label_2 Reset))))))

(event EventBeginPlay
  ;[1 1 1] Define Who is Player 01
  (if (> (.Y (Math|Vector|BreakVector (Transformation|GetActorLocation))) 0.0)
    (Variables|Default|SetPlayer01? true)
    ;[1 1 1] Default Animation Begin
    (Components|Animation|PlayAnimation (Variables|Character|GetMesh) "/Game/Fight_Game/Players/Char01/Animations/Char_Idle.Char_Idle" true)
    (else
      (Variables|Default|SetPlayer01? false))))

(fn ConstructionScript)

(fn CastFightGameMenu
  (bind _foundwidgets (Widget|GetAllWidgetsOfClass "/Game/Fight_Game/HUD/Widget_FightGame_Menu.Widget_FightGame_Menu_C" true))
  (bind _aswidget_fight_game_menu (Utilities|Casting|CastToWidget_FightGame_Menu (Utilities|Array|Get(acopy) _foundwidgets))
    (:then
      (return _aswidget_fight_game_menu))
    (:CastFailed
      (return _aswidget_fight_game_menu))))