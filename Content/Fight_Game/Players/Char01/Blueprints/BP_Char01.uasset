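; BP_Char01 is the playable fighting-game character, assigned to player one or two by its spawn Y position.
; Tick polls the menu widget to drive player two's costume color, ready poses and the switch to the AnimBP.
; Socket-attached fist and foot hitboxes trigger HitReaction on opponents during attacks.
; HitReaction looks up damage by hit type and updates the health UI, with death triggering ragdoll and winner declaration.
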(event OnComponentBeginOverlap(R_Punch)
  (params (OverlappedComponent :type Primitive%20Component%20Object%20Reference) (OtherActor :type Actor%20Object%20Reference) (OtherComp :type Primitive%20Component%20Object%20Reference) (OtherBodyIndex :type Integer) (bFromSweep :type Boolean) (SweepResult :type Hit%20Result%20Structure%20%28by%20ref%29))
  ;[1 1 1] Apply Damage
  (bind _enemyref (Utilities|CheckCollision OtherActor)
    (:Out
      (Variables|Default|SetEHitReaction "NewEnumerator0")
      (CallFunction|HitReaction _enemyref))))

(event OnComponentBeginOverlap(L_Punch)
  (params (OverlappedComponent :type Primitive%20Component%20Object%20Reference) (OtherActor :type Actor%20Object%20Reference) (OtherComp :type Primitive%20Component%20Object%20Reference) (OtherBodyIndex :type Integer) (bFromSweep :type Boolean) (SweepResult :type Hit%20Result%20Structure%20%28by%20ref%29))
  ;[1 1 1] Apply Damage
  (bind _enemyref (Utilities|CheckCollision OtherActor)
    (:Out
      (Variables|Default|SetEHitReaction "NewEnumerator2")
      (CallFunction|HitReaction _enemyref))))

(event OnComponentBeginOverlap(R_Foot)
  (params (OverlappedComponent :type Primitive%20Component%20Object%20Reference) (OtherActor :type Actor%20Object%20Reference) (OtherComp :type Primitive%20Component%20Object%20Reference) (OtherBodyIndex :type Integer) (bFromSweep :type Boolean) (SweepResult :type Hit%20Result%20Structure%20%28by%20ref%29))
  ;[1 1 1] Apply Damage
  (bind _enemyref (Utilities|CheckCollision OtherActor)
    (:Out
      (Variables|Default|SetEHitReaction "NewEnumerator1")
      (CallFunction|HitReaction _enemyref))))

(event OnComponentBeginOverlap(L_Foot)
  (params (OverlappedComponent :type Primitive%20Component%20Object%20Reference) (OtherActor :type Actor%20Object%20Reference) (OtherComp :type Primitive%20Component%20Object%20Reference) (OtherBodyIndex :type Integer) (bFromSweep :type Boolean) (SweepResult :type Hit%20Result%20Structure%20%28by%20ref%29))
  ;[1 1 1] Apply Damage
  (bind _enemyref (Utilities|CheckCollision OtherActor)
    (:Out
      (Variables|Default|SetEHitReaction "NewEnumerator3")
      (CallFunction|HitReaction _enemyref))))

(event Custom|Color
  ;[1 1 1] Change Color Costume
  (bind _returnvalue (Rendering|Material|CreateDynamicMaterialInstance (Variables|Character|GetMesh) 0 "/Game/Fight_Game/Players/Char01/Material/M_Char01.M_Char01" :!class /Script/Engine.PrimitiveComponent))
  (bind _output_get (Variables|Default|SetDynamicColor _returnvalue))
  (Rendering|Material|SetVectorParameterValue _output_get "BodyColor" "(R=1.000000,G=0.000000,B=0.000000,A=1.000000)" :!class /Script/Engine.MaterialInstanceDynamic))

(event Custom|Die
  (bind _returnvalue (Utilities|Name|MakeLiteralName "pelvis"))
  (bind _mesh (Variables|Character|GetMesh))
  ;[1 1 1] On Die
  (Utilities|FlowControl|DoOnce false
    (:Completed
      (Collision|SetCollisionEnabled (Variables|Collision|GetCapsuleComponent) "NoCollision")
      (Class|SkeletalMeshComponent|SetAllBodiesBelowPhysicsBlendWeight _mesh _returnvalue 1.0 false true)
      (Class|SkeletalMeshComponent|SetAllBodiesBelowSimulatePhysics _mesh _returnvalue true true)
      (Actor|Tick|SetActorTickEnabled false)
      (Default|DeclareWinner (Variables|Default|GetMainWidgetRef)))))

(event Custom|HitReaction
  (params (HitComponent :type Primitive%20Component%20Object%20Reference))
  (bind _attackdamagestruct (Variables|Default|GetAttackDamageStruct))
  (bind _ehitreaction (Variables|Default|GetEHitReaction))
  (bind _hitdamagepair (Utilities|Struct|BreakAttackDamageStruct _attackdamagestruct))
  ;[1 1 1] Receive Damage
  (if (not (Variables|Default|GetIsAttacked))
    (bind _keys (Utilities|Map|Keys _hitdamagepair))
    (bind _array_element (Utilities|Array|ForEachLoopwithBreak _keys :!label _label)
      (:LoopBody
        (if (Utilities|Enum|Equal(Enum) _array_element _ehitreaction)
          (Default|UpdateHealth (Variables|Default|GetMainWidgetRef) (Variables|Default|GetPlayer01?) (- (Variables|Default|GetHealth) (.Value (Utilities|Map|Find _hitdamagepair _ehitreaction))))
          (bind _output_get (Variables|Default|SetHealth (- (Variables|Default|GetHealth) (.Value (Utilities|Map|Find _hitdamagepair _ehitreaction)))))
          (if (<= _output_get 0.0)
            (CallFunction|Die)
            (goto _label Break)
            (else
              (Variables|Default|SetIsAttacked true)
              (goto _label Break))))))))

(event Custom|Disable%20Movement
  ;[1 1 1] Disabl_Navigtion_while_attacking
  (Variables|Default|SetAttack true))

(event Custom|ResetDie
  (bind _returnvalue (Utilities|Name|MakeLiteralName "pelvis"))
  (bind _mesh (Variables|Character|GetMesh))
  ;[1 1 1] On Die
  (Utilities|FlowControl|DoOnce false) ; enters at Reset
)

(event EventTick
  (params (DeltaSeconds :type Float%20%28single-precision%29))
  (bind _mesh (Variables|Character|GetMesh))
  (bind _charactermovement (Variables|Character|GetCharacterMovement))
  (bind _asfight_game_menu (CallFunction|CastFightGameMenu))
  (Utilities|FlowControl|Sequence
    (:then_0
      ;[1 1 1] Crouching - Stop and Restore Acceleration
      (if (AI|Components|NavMovement|IsCrouching _charactermovement)
        (Variables|/Script/Engine.CharacterMovementComponent|SetMaxAcceleration _charactermovement 0.0)
        (else
          (Variables|/Script/Engine.CharacterMovementComponent|SetMaxAcceleration _charactermovement 2048.0))))
    (:then_1
      ;[1 1 1] Change Color and Animations
      (if (Variables|/Game/Fight_Game/HUD/Widget_FightGame_Menu.Widget_FightGame_Menu_C|GetP2_ChangeColor _asfight_game_menu)
        (if (not (Variables|Default|GetPlayer01?))
          (if (Variables|/Game/Fight_Game/HUD/Widget_FightGame_Menu.Widget_FightGame_Menu_C|GetPlay_Game _asfight_game_menu)
            (Utilities|FlowControl|DoOnce false
              (:Completed
                (CallFunction|Color)))
            (else
              (CallFunction|Color))))))
    (:then_2
      (if (Variables|/Game/Fight_Game/HUD/Widget_FightGame_Menu.Widget_FightGame_Menu_C|GetP01_AnimReady _asfight_game_menu)
        (if (Variables|Default|GetPlayer01?)
          (Utilities|FlowControl|DoOnce false :!label _label
            (:Completed
              (Components|Animation|PlayAnimation (Variables|Character|GetMesh) "/Game/Fight_Game/Players/Char01/Animations/Char_Ready.Char_Ready" true))))))
    (:then_3
      (if (Variables|/Game/Fight_Game/HUD/Widget_FightGame_Menu.Widget_FightGame_Menu_C|GetP02_AnimReady _asfight_game_menu)
        (if (not (Variables|Default|GetPlayer01?))
          (goto _label))))
    (:then_4
      (if (Variables|/Game/Fight_Game/HUD/Widget_FightGame_Menu.Widget_FightGame_Menu_C|GetPlay_Game _asfight_game_menu)
        (Utilities|FlowControl|DoOnce false :!label _label_2
          (:Completed
            (Components|Animation|SetAnimationMode _mesh "AnimationBlueprint")
            (Components|SkeletalMesh|SetAnimInstanceClass _mesh "/Game/Fight_Game/Players/Char01/Blueprints/Char_AnimBP.Char_AnimBP_C")))
        (else
          (goto _label_2 Reset))))))

(event EventBeginPlay
  (Utilities|FlowControl|Sequence
    (:then_0
      ;[1 1 1] Define Who is Player 01
      (if (> (.Y (Math|Vector|BreakVector (Transformation|GetActorLocation))) 0.0)
        (Variables|Default|SetPlayer01? true)
        ;[1 1 1] Default Animation Begin
        (Components|Animation|PlayAnimation (Variables|Character|GetMesh) "/Game/Fight_Game/Players/Char01/Animations/Char_Idle.Char_Idle" true)
        (bind _asbp_global_controller (Utilities|Casting|CastToBP_Global_Controller (Game|GetPlayerController 0)))
        (Variables|Default|SetGlobalController _asbp_global_controller)
        (else
          (Variables|Default|SetPlayer01? false)
          (bind _asbp_global_controller_2 (Utilities|Casting|CastToBP_Global_Controller (Game|GetPlayerController 1)))
          (Variables|Default|SetGlobalController _asbp_global_controller_2))))
    (:then_1
      (if (Utilities|Enum|Equal(Enum) (Utilities|GetDisplayName self) "BP_Char01")
        (Actor|DestroyActor)))
    (:then_2
      (bind _foundwidgets (Widget|GetAllWidgetsOfClass "/Game/Fight_Game/HUD/Widget_FightGame_Menu.Widget_FightGame_Menu_C" false))
      (if (> (Utilities|Array|Length _foundwidgets) 1)
        (Development|PrintString "Too many widgets spawned" true true "(R=1.000000,G=0.048928,B=0.000000,A=1.000000)" 1e+01)
        (else
          (Variables|Default|SetMainWidgetRef (Utilities|Array|Get(acopy) _foundwidgets)))))))

(fn ConstructionScript
  (Transformation|AttachComponentToComponent (Variables|Default|GetR_Punch) (Variables|Character|GetMesh) "middle_01_r" "SnapToTarget" "SnapToTarget" "KeepRelative" true)
  (Transformation|AttachComponentToComponent (Variables|Default|GetL_Punch) (Variables|Character|GetMesh) "middle_01_l" "SnapToTarget" "SnapToTarget" "KeepRelative" true)
  (Transformation|AttachComponentToComponent (Variables|Default|GetR_Foot) (Variables|Character|GetMesh) "ball_r" "KeepRelative" "KeepRelative" "KeepRelative" true)
  (Transformation|AttachComponentToComponent (Variables|Default|GetL_Foot) (Variables|Character|GetMesh) "ball_l" "KeepRelative" "KeepRelative" "KeepRelative" true)
  (Transformation|AttachComponentToComponent (Variables|Default|GetR_Knee) (Variables|Character|GetMesh) "calf_r" "SnapToTarget" "SnapToTarget" "KeepRelative" true)
  (Transformation|AttachComponentToComponent (Variables|Default|GetL_Knee) (Variables|Character|GetMesh) "calf_l" "SnapToTarget" "SnapToTarget" "KeepRelative" true)
  (Transformation|AttachComponentToComponent (Variables|Default|GetR_Elbow) (Variables|Character|GetMesh) "lowerarm_r" "SnapToTarget" "SnapToTarget" "KeepRelative" true)
  (Transformation|AttachComponentToComponent (Variables|Default|GetL_Elbow) (Variables|Character|GetMesh) "lowerarm_l" "SnapToTarget" "SnapToTarget" "KeepRelative" true)
  (Transformation|AttachComponentToComponent (Variables|Default|GetHead) (Variables|Character|GetMesh) "head" "SnapToTarget" "SnapToTarget" "KeepRelative" true))

(fn CastFightGameMenu
  (bind _foundwidgets (Widget|GetAllWidgetsOfClass "/Game/Fight_Game/HUD/Widget_FightGame_Menu.Widget_FightGame_Menu_C" true))
  (bind _aswidget_fight_game_menu (Utilities|Casting|CastToWidget_FightGame_Menu (Utilities|Array|Get(acopy) _foundwidgets))
    (:then
      (return _aswidget_fight_game_menu))
    (:CastFailed
      (return _aswidget_fight_game_menu))))